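; BP_OLDLaneSpawner is a spawner actor that lays down a chain of BP_OLDLane street floor pieces at BeginPlay.
; A fixed-count loop places the first lane at the player pawn's location and each subsequent one at the newest lane's SpawnPoint.
; Each lane receives a reference back to the spawner, which tracks the newest lane to extend the chain.
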(event EventBeginPlay
  (CallFunction|SpawnInitialLane))

(event Collision|EventActorBeginOverlap
  (params (OtherActor :type Actor%20Object%20Reference)))

(event EventTick
  (params (DeltaSeconds :type Float%20%28single-precision%29)))

(fn ConstructionScript)

(fn SpawnLane
  (params (SpawnLocation :type Vector))
  (bind _returnvalue (Game|SpawnActorfromClass "/Game/Characters/Floors/street/BP_OLDLane.BP_OLDLane_C" (Math|Transform|MakeTransform SpawnLocation "0, 0, 0" "1.000000,1.000000,1.000000") "Undefined" 0 0))
  (bind _output_get (Variables|Default|SetNewestLane _returnvalue))
  (Variables|/Game/Characters/Floors/street/BP_OLDLane.BP_OLDLane_C|SetLaneSpawner _output_get self))

(fn SpawnLaneatSpawnPoint
  (CallFunction|SpawnLane (Transformation|GetWorldLocation (Variables|/Game/Characters/Floors/street/BP_OLDLane.BP_OLDLane_C|GetSpawnPoint (Variables|Default|GetNewestLane)))))

(fn SpawnInitialLane
  (for _index (range 0 23)
    (Utilities|IsValid (Variables|Default|GetNewestLane)
      (:Is%20Valid
        (CallFunction|SpawnLaneatSpawnPoint))
      (:Is%20Not%20Valid
        (CallFunction|SpawnLane (Transformation|GetActorLocation (Game|Player|GetPlayerPawn 0)))))))