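; BP_River is a river floor piece that spawns drifting logs and drowns the chicken that falls in.
; On BeginPlay it picks one of two spawn points, fixing the log direction, and starts a randomized-interval looping timer that spawns BP_Log on a coin flip.
; Two trigger volumes destroy logs.
; One-shot overlaps update the chicken's step count, or call Drown and play a splash sound.
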(event OnComponentBeginOverlap(CollisionSteps)
  (params (OverlappedComponent :type Primitive%20Component%20Object%20Reference) (OtherActor :type Actor%20Object%20Reference) (OtherComp :type Primitive%20Component%20Object%20Reference) (OtherBodyIndex :type Integer) (bFromSweep :type Boolean) (SweepResult :type Hit%20Result%20Structure%20%28by%20ref%29))
  (bind _asbp_chicken (Utilities|Casting|CastToBP_Chicken OtherActor))
  (Utilities|FlowControl|DoOnce false
    (:Completed
      (Default|UpdateMyStep _asbp_chicken))))

(event OnComponentBeginOverlap(Destroy)
  (params (OverlappedComponent :type Primitive%20Component%20Object%20Reference) (OtherActor :type Actor%20Object%20Reference) (OtherComp :type Primitive%20Component%20Object%20Reference) (OtherBodyIndex :type Integer) (bFromSweep :type Boolean) (SweepResult :type Hit%20Result%20Structure%20%28by%20ref%29))
  (bind _asbp_log (Utilities|Casting|CastToBP_Log OtherActor))
  (Actor|DestroyActor _asbp_log))

(event OnComponentBeginOverlap(Destroy1)
  (params (OverlappedComponent :type Primitive%20Component%20Object%20Reference) (OtherActor :type Actor%20Object%20Reference) (OtherComp :type Primitive%20Component%20Object%20Reference) (OtherBodyIndex :type Integer) (bFromSweep :type Boolean) (SweepResult :type Hit%20Result%20Structure%20%28by%20ref%29))
  (bind _asbp_log (Utilities|Casting|CastToBP_Log OtherActor))
  (Actor|DestroyActor _asbp_log))

(event OnComponentBeginOverlap(Drown)
  (params (OverlappedComponent :type Primitive%20Component%20Object%20Reference) (OtherActor :type Actor%20Object%20Reference) (OtherComp :type Primitive%20Component%20Object%20Reference) (OtherBodyIndex :type Integer) (bFromSweep :type Boolean) (SweepResult :type Hit%20Result%20Structure%20%28by%20ref%29))
  (bind _asbp_chicken (Utilities|Casting|CastToBP_Chicken OtherActor))
  (Utilities|FlowControl|DoOnce false
    (:Completed
      (Default|Drown _asbp_chicken)
      (Audio|PlaySoundatLocation "/Game/Audio/splash_Cue.splash_Cue" (Transformation|GetActorLocation) "0, 0, 0" 1.0 1.0 0.0 0 0 0 0))))

(event Custom|Spawn%20Different%20Cars
  (if (Math|Random|RandomBool)
    (if (Variables|Default|GetOneCarSpawn)
      (Game|SpawnActorfromClass "/Game/Characters/Floors/Blueprints/BP_Log.BP_Log_C" (Math|Transform|MakeTransform (Variables|Default|GetBeginSpawn) "0,90.000000, 0" "1.000000,1.000000,0.600000") "Undefined" 0 0)
      (else
        (Game|SpawnActorfromClass "/Game/Characters/Floors/Blueprints/BP_Log.BP_Log_C" (Math|Transform|MakeTransform (Variables|Default|GetStopSpawn) "0,-90.000000, 0" "1.000000,1.000000,0.600000") "Undefined" 0 0)))))

(event EventBeginPlay
  (Variables|Default|SetBeginSpawn (Transformation|GetWorldLocation (Variables|Default|GetSpawnSTUFF)))
  (Variables|Default|SetStopSpawn (Transformation|GetWorldLocation (Variables|Default|GetSpawnSTUFF2)))
  (Variables|Default|SetOneCarSpawn (Math|Random|RandomBool))
  (Utilities|Time|SetTimerbyEvent (delegate Custom|Spawn%20Different%20Cars) (Math|Random|RandomFloatinRange 1.5 2.0) true))

(fn ConstructionScript)