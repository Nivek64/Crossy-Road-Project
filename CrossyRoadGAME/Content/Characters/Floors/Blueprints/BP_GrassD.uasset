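; BP_GrassD is a grass floor piece that scatters obstacles and coins and registers the chicken's step on it.
; On BeginPlay it walks fixed slots along Y between two marker components, randomly spawning a BP_RockTree and a BP_Coin at the same point.
; Collision handling nudges or skips overlapping spawns.
; The first BP_Chicken hit on GrassL calls UpdateMyStep, gated by DoOnce so it counts once.
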(event OnComponentHit(GrassL)
  (params (HitComponent :type Primitive%20Component%20Object%20Reference) (OtherActor :type Actor%20Object%20Reference) (OtherComp :type Primitive%20Component%20Object%20Reference) (NormalImpulse :type Vector :default "0, 0, 0") (Hit :type Hit%20Result%20Structure%20%28by%20ref%29))
  (bind _asbp_chicken (Utilities|Casting|CastToBP_Chicken OtherActor))
  (Utilities|FlowControl|DoOnce false
    (:Completed
      (Default|UpdateMyStep _asbp_chicken))))

(event EventBeginPlay
  (Variables|Default|SetBeginSpawn (Transformation|GetWorldLocation (Variables|Default|GetspawnSTUFF)))
  (Variables|Default|SetStopSpawn (Transformation|GetWorldLocation (Variables|Default|GetspawnSTUFF2)))
  (for _index (range 0 (Math|Float|Truncate (/ (Math|Vector|Distance(Vector) (Variables|Default|GetBeginSpawn) (Variables|Default|GetStopSpawn)) 85.0)))
    (if (> (Math|Random|RandomFloat) 0.8)
      (Game|SpawnActorfromClass "/Game/Characters/Floors/Blueprints/BP_RockTree.BP_RockTree_C" (Math|Transform|MakeTransform (Math|Vector|MakeVector (.x (Variables|Default|GetBeginSpawn)) (+ (* _index 90) (.Y (Math|Vector|BreakVector (Variables|Default|GetBeginSpawn)))) (.z (Variables|Default|GetBeginSpawn))) "0, 0, 0" "1.000000,1.000000,1.000000") "AdjustIfPossibleButDontSpawnIfColliding" 0 0)
      (Game|SpawnActorfromClass "/Game/Characters/Floors/Blueprints/BP_Coin.BP_Coin_C" (Math|Transform|MakeTransform (Math|Vector|MakeVector (.x (Variables|Default|GetBeginSpawn)) (+ (* _index 90) (.Y (Math|Vector|BreakVector (Variables|Default|GetBeginSpawn)))) (.z (Variables|Default|GetBeginSpawn))) "0, 0, 0" "1.000000,1.000000,1.000000") "AdjustIfPossibleButDontSpawnIfColliding" 0 0))))

(fn ConstructionScript)