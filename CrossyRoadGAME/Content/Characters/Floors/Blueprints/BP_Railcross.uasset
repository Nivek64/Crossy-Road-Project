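; BP_Railcross is a railroad crossing actor whose two signal lights flash alternately.
; Tick increments a frame counter and, on reaching ten, resets it and toggles LeftLightOn, swapping intensity between LightLeft and LightRight.
; The blink rate depends on frame rate, as the counter ignores delta time.
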(event EventBeginPlay
  (Variables|Default|SetLeftLightOn false))

(event Collision|EventActorBeginOverlap
  (params (OtherActor :type Actor%20Object%20Reference)))

(event EventTick
  (params (DeltaSeconds :type Float%20%28single-precision%29))
  (if (>= (Variables|Default|GetCounter) 10)
    (Variables|Default|SetCounter 0)
    (if (Variables|Default|GetLeftLightOn)
      (Rendering|Components|Light|SetIntensity (Variables|Default|GetLightLeft) 0.0)
      (Rendering|Components|Light|SetIntensity (Variables|Default|GetLightRight) 1e+04)
      (Variables|Default|SetLeftLightOn false)
      (else
        (Rendering|Components|Light|SetIntensity (Variables|Default|GetLightLeft) 1e+04)
        (Rendering|Components|Light|SetIntensity (Variables|Default|GetLightRight) 0.0)
        (Variables|Default|SetLeftLightOn true)))
    (else
      (Variables|Default|SetCounter (+ (Variables|Default|GetCounter) 1)))))

(fn ConstructionScript)