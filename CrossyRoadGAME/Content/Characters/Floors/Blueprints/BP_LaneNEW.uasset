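; BP_LaneNEW is a lane floor actor that spawns BP_OrangeCar traffic from one of its two ends.
; On BeginPlay it caches both spawn marker locations, picks a random end for its lifetime and starts a looping timer with a randomized interval, rolled once.
; Each tick of that timer has a random chance to spawn a car at the chosen end, with opposite rotations for the two ends.
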(event Custom|Spawn%20Different%20Cars
  (if (Math|Random|RandomBool)
    (if (Variables|Default|GetOneCarSpawn)
      (Game|SpawnActorfromClass "/Game/Characters/Floors/Blueprints/BP_OrangeCar.BP_OrangeCar_C" (Math|Transform|MakeTransform (Variables|Default|GetBeginSpawn) "0,90.000000, 0" "1.000000,1.000000,1.000000") "AdjustIfPossibleButAlwaysSpawn" 0 0)
      (else
        (Game|SpawnActorfromClass "/Game/Characters/Floors/Blueprints/BP_OrangeCar.BP_OrangeCar_C" (Math|Transform|MakeTransform (Variables|Default|GetStopSpawn) "0,-90.000000, 0" "1.000000,1.000000,1.000000") "AdjustIfPossibleButAlwaysSpawn" 0 0)))))

(event EventBeginPlay
  (Variables|Default|SetBeginSpawn (Transformation|GetWorldLocation (Variables|Default|GetSpawnSTUFF)))
  (Variables|Default|SetStopSpawn (Transformation|GetWorldLocation (Variables|Default|GetSpawnSTUFF2)))
  (Variables|Default|SetOneCarSpawn (Math|Random|RandomBool))
  (Utilities|Time|SetTimerbyEvent (delegate Custom|Spawn%20Different%20Cars) (Math|Random|RandomFloatinRange 2.0 3.0) true))

(fn ConstructionScript)