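; BP_OrangeCar is a projectile-movement car hazard that kills the chicken character on overlap, limited by a DoOnce.
; On BeginPlay a random roll either keeps the default car or turns it into a blue variant with its own speed and a respawned attached driving sound.
; A separate honk trigger box plays an attached horn when the chicken enters, gated by a DoOnce that resets after a short delay.
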(event OnComponentBeginOverlap(Collision)
  (params (OverlappedComponent :type Primitive%20Component%20Object%20Reference) (OtherActor :type Actor%20Object%20Reference) (OtherComp :type Primitive%20Component%20Object%20Reference) (OtherBodyIndex :type Integer) (bFromSweep :type Boolean) (SweepResult :type Hit%20Result%20Structure%20%28by%20ref%29))
  ;[1 0.3339 0.2442] Kill player
  (bind _asbp_chicken (Utilities|Casting|CastToBP_Chicken OtherActor))
  (Utilities|FlowControl|DoOnce false
    (:Completed
      (Default|KilledbyCar _asbp_chicken))))

(event OnComponentBeginOverlap(Box_Honk)
  (params (OverlappedComponent :type Primitive%20Component%20Object%20Reference) (OtherActor :type Actor%20Object%20Reference) (OtherComp :type Primitive%20Component%20Object%20Reference) (OtherBodyIndex :type Integer) (bFromSweep :type Boolean) (SweepResult :type Hit%20Result%20Structure%20%28by%20ref%29))
  ;[0.7873 1 0.7365] Audio
  (Utilities|Casting|CastToBP_Chicken OtherActor)
  (Utilities|FlowControl|DoOnce false :!label _label
    (:Completed
      (Audio|Components|Audio|FadeOut (Variables|Default|Getcar_horn_Cue) 0.0 0.0 "Linear" :!class /Script/Engine.AudioComponent)
      (Audio|SpawnSoundAttached "/Game/Audio/car_horn_Cue.car_horn_Cue" (Variables|Default|GetOrangeCar) "None" (Transformation|GetActorLocation) "0, 0, 0" "SnapToTarget" false 1.0 1.0 0.0 0 0)
      (Utilities|FlowControl|Delay 0.1)
      (goto _label Reset))))

(event EventBeginPlay
  (bind _orangecar (Variables|Default|GetOrangeCar))
  (bind _projectilemovement (Variables|Default|GetProjectileMovement))
  ;[1 0.295 0.6964] Spawn 2 cars
  (switch int (Math|Random|RandomIntegerinRange 0 1)
    (:1
      (Variables|/Script/Engine.ProjectileMovementComponent|SetInitialSpeed _projectilemovement 575.0)
      (Variables|/Script/Engine.ProjectileMovementComponent|SetMaxSpeed _projectilemovement 575.0)
      (Components|StaticMesh|SetStaticMesh _orangecar "/Game/Characters/Vehicles/Cars/BlueCar.BlueCar")
      (Audio|Components|Audio|FadeOut (Variables|Default|GetDriving_Cue) 0.0 0.0 "Linear" :!class /Script/Engine.AudioComponent)
      (Audio|SpawnSoundAttached "/Game/Audio/Car_Driving_Cue.Car_Driving_Cue" _orangecar "None" (Transformation|GetActorLocation) "0, 0, 0" "KeepWorldPosition" false 1.0 1.0 0.0 0 0))))

(fn ConstructionScript)