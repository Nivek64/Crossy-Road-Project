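; Player chicken character for a hopping game with coins, cars and drowning, in the style of Crossy Road.
; Axis input launches cooldown-gated hops with a cluck, while per-direction timelines turn the mesh to face travel.
; It creates the HUD, tracks coins and steps, and destroys overlapped coins.
; Car hits flatten the chicken; they and drowning block input and share a one-shot game-over screen.
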(event Custom|DoCooldownJump
  ;[0 0.1746 1] Movement
  (Utilities|FlowControl|DoOnce false :!label _label
    (:Completed
      (Variables|Default|SetCheckJump false)
      (Utilities|FlowControl|Delay 0.3)
      (Variables|Default|SetCheckJump true)
      (goto _label Reset))))

(event Custom|UpdateMyStep
  ;[0.4247 1 0.3851] Step counter
  (bind _result (Math|Float|IncrementFloat (Variables|Default|GetSteps))
    (:%20%20
      (Variables|Default|SetSteps _result))))

(event Custom|UpdateCoins
  ;[1 1 1] coin audio
  (bind _result (Math|Float|IncrementFloat (Variables|Default|GetCoins))
    (:%20%20
      (Variables|Default|SetCoins _result)
      (Audio|PlaySoundatLocation "/Game/Audio/Coin_Sound_Cue.Coin_Sound_Cue" "0, 0, 0" "0, 0, 0" 1.0 1.0 0.0 0 0 0 0))))

(event Custom|KilledByCar
  (bind _charactermovement (Variables|Character|GetCharacterMovement))
  ;[1 0 0] HUD Gameover
  (Variables|Default|SetIsDead true)
  (Transformation|SetWorldScale3D (Variables|Default|GetChicken) "0.500000,0.500000,0.025000")
  (Utilities|FlowControl|DoOnce false
    (:Completed
      (bind _returnvalue (UserInterface|CreateWidget "/Game/UI/WBP_GameOver.WBP_GameOver_C"))
      (UserInterface|Viewport|AddtoViewport _returnvalue 0)
      (Variables|/Script/Engine.PlayerController|SetbShowMouseCursor (Game|GetPlayerController 0) true)
      (Variables|/Script/Engine.CharacterMovementComponent|SetMaxAcceleration _charactermovement 0.0)
      (Variables|/Script/Engine.CharacterMovementComponent|SetMaxWalkSpeed _charactermovement 0.0))))

(event Custom|Drown
  (bind _charactermovement (Variables|Character|GetCharacterMovement))
  ;[1 0 0] HUD Gameover
  (Variables|Default|SetIsDead true)
  (Utilities|FlowControl|DoOnce false
    (:Completed
      (bind _returnvalue (UserInterface|CreateWidget "/Game/UI/WBP_GameOver.WBP_GameOver_C"))
      (UserInterface|Viewport|AddtoViewport _returnvalue 0)
      (Variables|/Script/Engine.PlayerController|SetbShowMouseCursor (Game|GetPlayerController 0) true)
      (Variables|/Script/Engine.CharacterMovementComponent|SetMaxAcceleration _charactermovement 0.0)
      (Variables|/Script/Engine.CharacterMovementComponent|SetMaxWalkSpeed _charactermovement 0.0))))

(event EventBeginPlay
  ;[1 1 1] Player HUD
  (bind _returnvalue (UserInterface|CreateWidget "/Game/UI/WBP_HUD.WBP_HUD_C"))
  (UserInterface|Viewport|AddtoViewport _returnvalue 0))

(event Collision|EventActorBeginOverlap
  (params (OtherActor :type Actor%20Object%20Reference))
  ;[1 1 1] destroy coin
  (bind _asbp_coin (Utilities|Casting|CastToBP_Coin OtherActor))
  (Actor|DestroyActor _asbp_coin))

(event Input|AxisEvents|InputAxisMoveRight
  (params (AxisValue :type Float%20%28single-precision%29))
  (bind _chicken (Variables|Default|GetChicken))
  (bind _chicken_2 (Variables|Default|GetChicken))
  ;[0 0.1746 1] Movement
  (if (not (Variables|Default|GetIsDead))
    (if (and (> (Math|Float|Absolute(Float) AxisValue) 0.3) (Variables|Default|GetCheckJump))
      (CallFunction|DoCooldownJump)
      (Character|LaunchCharacter (Math|Vector|MakeVector 0.0 (* AxisValue 975.0) 1e+03) true true)
      (Audio|PlaySoundatLocation "/Game/Audio/chicken_cluck_Cue.chicken_cluck_Cue" "0, 0, 0" "0, 0, 0" 1.0 1.0 0.0 0 0 0 0)
      (if (> AxisValue 0.3)
        (bind _checkrotation (Timeline|Timeline%20of%20Chicken%20Movement%28Right%29 PlayFromStart)
          (:Update
            (Transformation|SetWorldRotation _chicken_2 (Math|Rotator|Lerp(Rotator) (Transformation|GetWorldRotation _chicken_2) "0, 0, 0" _checkrotation true) false false)))
        (else
          (bind _checkrotation_2 (Timeline|Timeline%20of%20Chicken%20Movement%28Left%29 PlayFromStart)
            (:Update
              (Transformation|SetWorldRotation _chicken (Math|Rotator|Lerp(Rotator) (Transformation|GetWorldRotation _chicken) "0,-180.000000, 0" _checkrotation_2 true) false false))))))))

(event Input|AxisEvents|InputAxisMoveForward
  (params (AxisValue :type Float%20%28single-precision%29))
  (bind _chicken (Variables|Default|GetChicken))
  (bind _chicken_2 (Variables|Default|GetChicken))
  ;[0 0.1746 1] Movement
  (if (not (Variables|Default|GetIsDead))
    (if (and (> (Math|Float|Absolute(Float) AxisValue) 0.3) (Variables|Default|GetCheckJump))
      (CallFunction|DoCooldownJump)
      (Character|LaunchCharacter (Math|Vector|MakeVector (* AxisValue 1.1e+03) 0.0 1e+03) true true)
      (Audio|PlaySoundatLocation "/Game/Audio/chicken_cluck_Cue.chicken_cluck_Cue" "0, 0, 0" "0, 0, 0" 1.0 1.0 0.0 0 0 0 0)
      (if (> AxisValue 0.3)
        (bind _checkrotation (Timeline|Timeline%20of%20Chicken%20Movement%28Forward%29 PlayFromStart)
          (:Update
            (Transformation|SetWorldRotation _chicken (Math|Rotator|Lerp(Rotator) (Transformation|GetWorldRotation _chicken) "0,-90.000000, 0" _checkrotation true) false false)))
        (else
          (bind _checkrotation_2 (Timeline|Timeline%20of%20Chicken%20Movement%28Backward%29 PlayFromStart)
            (:Update
              (Transformation|SetWorldRotation _chicken_2 (Math|Rotator|Lerp(Rotator) (Transformation|GetWorldRotation _chicken_2) "0,90.000000, 0" _checkrotation_2 true) false false))))))))

(fn ConstructionScript)